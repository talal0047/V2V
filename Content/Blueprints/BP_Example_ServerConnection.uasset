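; Example actor that lets players host or join a direct-IP multiplayer session through a simple connection menu.
; On BeginPlay it requests the external IP via V2V, waits briefly, then shows WBP_ExampleUI with that IP and binds its Host and Join buttons.
; Hosting optionally tries UPnP port forwarding, flagging failure in the UI, then starts a listen server regardless.
; Joining connects to the entered IP, and game shutdown ends the UPnP mapping.
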(event Custom|OnHostButtonClicked
  (params (Enable%20Upnp :type Boolean))
  (if Enable%20Upnp
    (bind _isupnpsuccessfull (Class|V2VComponent|TryActivatingUpnp (Variables|Default|GetV2V) 7777))
    (if _isupnpsuccessfull
      _
      (else
        (Default|OnUpnpFailure (Variables|Default|GetExampleUI_Ref))
        (Utilities|FlowControl|Delay 2.5))))
  (Class|V2VComponent|HostServer (Game|GetGameInstance) "MotionControllerMap" 7777 true false))

(event Custom|OnGameShutdown
  (Class|V2VComponent|EndUpnpActivation (Variables|Default|GetV2V)))

(event Custom|JoinButtonClicked
  (params (ip :type String))
  (Class|V2VComponent|JoinServer (Game|GetGameInstance) ip))

(event EventBeginPlay
  (bind _v2v (Variables|Default|GetV2V))
  (Class|V2VComponent|GetExternalIP _v2v)
  (Utilities|FlowControl|Delay 1.5)
  (bind _output_get (Variables|Default|SetExternalIp (Variables|/Script/V2V.V2VComponent|GetExternalIP _v2v)))
  (bind _returnvalue (UserInterface|CreateWidget "/V2V/WIdget/WBP_ExampleUI.WBP_ExampleUI_C" (Game|GetPlayerController 0) _output_get))
  (bind _output_get_2 (Variables|Default|SetExampleUI_Ref _returnvalue))
  (UserInterface|Viewport|AddtoViewport _output_get_2 0)
  (EventDispatchers|BindEventtoOnHostButtonClicked _output_get_2 (EventDispatchers|CreateEvent :!event Custom|OnHostButtonClicked))
  (EventDispatchers|BindEventtoOnJoinButtonClicked _output_get_2 (EventDispatchers|CreateEvent :!event Custom|JoinButtonClicked)))

(fn ConstructionScript)