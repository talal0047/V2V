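; BP_Example_KickPlayerMenuController sets up an example kick-player menu on the authority side, for both VR and flat-screen play.
; In VR it takes the WBP_KickPlayerUI widget from a BP_Example_VR_KickPlayerMenu actor in the level.
; Otherwise it creates that widget hidden in the viewport, where Tab toggles its visibility and refreshes the list each time it opens.
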(event EventBeginPlay
  ;[0.15 0.15 0.15 0.5] Init
  (Networking|SwitchHasAuthority
    (:Authority
      (if (Variables|Default|GetisVr)
        (bind _returnvalue (Actor|GetActorOfClass "/V2V/Blueprints/BP_Example_VR_KickPlayerMenu.BP_Example_VR_KickPlayerMenu_C"))
        (bind _aswbp_kick_player_ui (Utilities|Casting|CastToWBP_KickPlayerUI (UserInterface|GetWidget (Variables|/V2V/Blueprints/BP_Example_VR_KickPlayerMenu.BP_Example_VR_KickPlayerMenu_C|GetWidget _returnvalue))))
        (Variables|Default|SetWB%20Kick%20Player%20Menu _aswbp_kick_player_ui)
        (else
          (bind _returnvalue_2 (UserInterface|CreateWidget "/V2V/WIdget/WBP_KickPlayerUI.WBP_KickPlayerUI_C" (Game|GetPlayerController 0)))
          (bind _output_get (Variables|Default|SetWB%20Kick%20Player%20Menu _returnvalue_2))
          (UserInterface|Viewport|AddtoViewport _output_get 0)
          (Variables|/Script/UMG.Widget|SetVisibility (Variables|Default|GetWB%20Kick%20Player%20Menu) "Hidden"))))))

(event Input|KeyboardEvents|Tab
  (params (Key :type Key%20Structure :default "None"))
  (bind _wb_kick_player_menu (Variables|Default|GetWB%20Kick%20Player%20Menu))
  ;[0.15 0 0.1251 0.5] Toggle Kick Player Menu Visibility
  (:Pressed
    (if (not (Variables|Default|GetisVr))
      (Utilities|FlowControl|FlipFlop
        (:A
          (Variables|/Script/UMG.Widget|SetVisibility _wb_kick_player_menu "Visible")
          (Default|RefreshList _wb_kick_player_menu))
        (:B
          (Variables|/Script/UMG.Widget|SetVisibility _wb_kick_player_menu "Hidden"))))))

(fn ConstructionScript)