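; BPC_V2VPlayerSessionController is a Blueprint component that tracks connected players and supports kicking them from the session.
; Login and logout events keep PlayersArray current, adding each new player uniquely and removing those who leave.
; KickPlayerByIndex prints a debug message, kicks the player at the given array index with a text reason, and removes them from the array if the kick succeeds.
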(event Custom|OnLogout
  (params (LoggedOutPlayer :type Player%20Controller%20Object%20Reference))
  ;[0.15 0.15 0.15 0.5] On Player Logout
  (Utilities|Array|RemoveItem (Variables|Default|GetPlayersArray) LoggedOutPlayer))

(event Custom|KickPlayerByIndex
  (params (PlayerIndex :type Integer) (Reason :type String))
  (bind _playersarray (Variables|Default|GetPlayersArray))
  (bind _output (Utilities|Array|Get(acopy) _playersarray PlayerIndex))
  ;[0.15 0 0 0.5] Kick Player Functionality
  (Development|PrintString (Utilities|String|Append (Utilities|String|ToString(Integer) PlayerIndex) " Kick initiated"))
  (bind _returnvalue (Class|AdvancedSessionsLibrary|KickPlayer _output (Utilities|Text|ToText(String) Reason)))
  (if _returnvalue
    (Utilities|Array|RemoveItem (Variables|Default|GetPlayersArray) _output)))

(event Custom|OnPostLogin
  (params (NewPlayer :type Player%20Controller%20Object%20Reference))
  ;[0.15 0.15 0.15 0.5] On Player Join
  (Utilities|Array|AddUnique (Variables|Default|GetPlayersArray) NewPlayer))